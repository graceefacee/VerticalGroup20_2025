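; BP_Bed is an interactable bed that lets the player sleep to advance to the next day.
; An overlap box shows a name prompt and sets CanSleep for the first-person character.
; Interact plays a fade, sets the DaySequence time to morning, increments the day on the player's display and calls OnPlayerSleep.
; Sleeping through the final day opens the win map.
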(event `self.ReceiveBeginPlay`
  (`self.getBed`)
  (set `self.DaySequenceRef` (`DaySequenceSubsystem.GetDaySequenceActor` (subsystem `DaySequenceSubsystem`) true)))

(event `self.InteractBox.OnComponentBeginOverlap`
  (params (OverlappedComponent :type "PrimitiveComponent Object Reference") (OtherActor :type "Actor Object Reference") (OtherComp :type "PrimitiveComponent Object Reference") (OtherBodyIndex :type Integer) (bFromSweep :type Boolean) (SweepResult :type "HitResult Structure (by ref)"))
  ;[1 0.3388 0.6589 0.5] Overlap pop up text
  (if (== (`GameplayStatics.GetObjectClass` OtherActor) "/Game/FirstPerson/Blueprints/BP_FirstPersonCharacter.BP_FirstPersonCharacter_C")
    (set `self.CanSleep` true)
    (bind _aswbp_pick_up (cast `/Game/DarcyBlueprints/UI/WBP_PickUp` (`WidgetComponent.GetWidget` (`self.InteractPrompt`))))
    (`/Game/DarcyBlueprints/UI/WBP_PickUp.updateName` _aswbp_pick_up (`self.Bed Text`))
    (`SceneComponent.SetVisibility` (`self.InteractPrompt`) true false)))

(event `self.InteractBox.OnComponentEndOverlap`
  (params (OverlappedComponent :type "PrimitiveComponent Object Reference") (OtherActor :type "Actor Object Reference") (OtherComp :type "PrimitiveComponent Object Reference") (OtherBodyIndex :type Integer))
  ;[1 0.3388 0.6589 0.5] Overlap pop up text
  (set `self.CanSleep` false)
  (`SceneComponent.SetVisibility` (`self.InteractPrompt`) false false))

(event `winGameOver`
  ;[1 0.3388 0.6589 0.5] Win Game Over
  (`GameplayStatics.OpenLevel` "WonEndMap"))

(event `/Game/DarcyBlueprints/BPI_Interact.Interact`
  (params (Interactor :type "Actor Object Reference"))
  (bind _returnvalue (`|CreateWidget` "/Game/WBP_Fade.WBP_Fade_C" (`GameplayStatics.GetPlayerController` 0)))
  (`UserWidget.AddToViewport` _returnvalue 0)
  (`/Game/WBP_Fade.PlayFade` _returnvalue)
  (`DaySequenceActor.SetTimeOfDay` (`self.DaySequenceRef`) 8.0)
  (bind _asbp_first_person_character (cast `/Game/FirstPerson/Blueprints/BP_FirstPersonCharacter` (`GameplayStatics.GetPlayerCharacter` 0)))
  (bind _output_get (set `self.DayNumber` (+ (`KismetMathLibrary.Clamp` (`self.DayNumber`) 1 6) 1)))
  ;[0.8058 0.2778 0.5445 0.5] Added FPC Integration
  (`/Game/WBP_DayDisplay.SetDayNumber` (`/Game/FirstPerson/Blueprints/BP_FirstPersonCharacter.DayDisplayWidget` _asbp_first_person_character) _output_get)
  (bind _day (`self.updateDay`))
  (`self.onPlayerSleep`)
  (if (> _day 6)
    (`self.winGameOver`)))

(fn `getBed`
  (returns (bed :type "/Game/BP_Bed Object Reference"))
  (return self))

(fn `updateDay`
  (returns (day :type Integer))
  (return (`self.DayNumber`)))

(fn `UserConstructionScript`)