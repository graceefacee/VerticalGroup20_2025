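; Base actor for a wellness "factor" that tool effects raise or lower, killing the player at zero.
; Wellness changes show +, - or MAX widgets and swap small, medium or large meshes from the FactorInfo data asset by threshold.
; Player dispatchers toggle a depletion timer affecting "Main" actors, while BP_Bed's day sets limits at BeginPlay and, on sleep, depletion rate.
; "Tutorial" actors unlock BP_TutorialFish dialogue at maximum wellness.
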(event `/Game/DarcyBlueprints/BPI_UpdateFactor.modifyWellness`
  (params (value :type "Float (double-precision)"))
  ;[1 0.3388 0.6589 0.5] Gets value from tool, then modifys wellness in response
  (if (not (`self.dead`))
    (set `self.playerFire` true)
    (set `self.initialWellness` (`self.wellness`))
    (bind _output_get (set `self.effect` value))
    (set `self.wellness` (`KismetMathLibrary.FClamp` (+ _output_get (`self.initialWellness`)) (`self.minWellness`) (`self.maxWellness`)))
    (`self.updateEffectText`)
    (`self.updateThreshold`)
    (if (== (`self.wellness`) 0.0)
      (bind _returnvalue (`GameplayStatics.GetActorOfClass` "/Game/FirstPerson/Blueprints/BP_FirstPersonCharacter.BP_FirstPersonCharacter_C"))
      (`/Game/FirstPerson/Blueprints/BP_FirstPersonCharacter.OnDead` _returnvalue)
      (set `self.dead` true))
    (set `self.playerFire` false)
    (if (and (`self.ActorHasTag` "Tutorial") (== (`self.wellness`) (`self.maxWellness`)))
      (`self.updateLockedDialogue`))))

(event `updateEffectText`
  (bind _poseffecttext (`self.PosEffectText`))
  (bind _maxwellnesstext (`self.MaxWellnessText`))
  (bind _negeffecttext (`self.NegEffectText`))
  ;[1 0.3388 0.6589 0.5] Updates the +, -, MAX effect depending on tool effect
  (if (< (`self.wellness`) (`self.initialWellness`))
    (`SceneComponent.SetVisibility` _negeffecttext true false)
    (bind _aswbp_neg_effect (cast `/Game/DarcyBlueprints/UI/WBP_NegEffect` (`WidgetComponent.GetWidget` _negeffecttext)))
    (`UserWidget.PlayAnimation` _aswbp_neg_effect (`/Game/DarcyBlueprints/UI/WBP_NegEffect.fadeOut` _aswbp_neg_effect) 0.0 1 "Forward" 1.0 false)
    (`KismetSystemLibrary.Delay` 1.0)
    (`SceneComponent.SetVisibility` (`self.NegEffectText`) false false)
    (elif (> (`self.wellness`) (`self.initialWellness`))
      (`SceneComponent.SetVisibility` _poseffecttext true false)
      (bind _aswbp_pos_effect (cast `/Game/DarcyBlueprints/UI/WBP_PosEffect` (`WidgetComponent.GetWidget` _poseffecttext)))
      (`UserWidget.PlayAnimation` _aswbp_pos_effect (`/Game/DarcyBlueprints/UI/WBP_PosEffect.fadeOut` _aswbp_pos_effect) 0.0 1 "Forward" 1.0 false)
      (`KismetSystemLibrary.Delay` 1.0)
      (`SceneComponent.SetVisibility` (`self.PosEffectText`) false false)
      (elif (== (`self.wellness`) (`self.maxWellness`))
        (`SceneComponent.SetVisibility` _maxwellnesstext true false)
        (bind _aswbp_max_effect (cast `/Game/DarcyBlueprints/UI/WBP_MaxEffect` (`WidgetComponent.GetWidget` _maxwellnesstext)))
        (`UserWidget.PlayAnimation` _aswbp_max_effect (`/Game/DarcyBlueprints/UI/WBP_MaxEffect.fadeOut` _aswbp_max_effect) 0.0 1 "Forward" 1.0 false)
        (`KismetSystemLibrary.Delay` 1.0)
        (`SceneComponent.SetVisibility` (`self.MaxWellnessText`) false false)))))

(event `updateLockedDialogue`
  ;[1 0.3388 0.6589 0.5] Unlocks dialogue options
  (bind _returnvalue (`GameplayStatics.GetActorOfClass` "/Game/DarcyBlueprints/Tutorial/BP_TutorialFish.BP_TutorialFish_C"))
  (`/Game/DarcyBlueprints/Tutorial/BP_TutorialFish.dialogueUnlocked` _returnvalue))

(event `handleDepletionStop`
  ;[1 0.3388 0.6589 0.5] Depletion Event Binding
  (`self.stopWellnessDepletion`))

(event `handleWellnessDepletion`
  ;[1 0.3388 0.6589 0.5] Depletion Event Binding
  (`self.startWellnessDepletion`))

(event `startWellnessDepletion`
  ;[1 0.3388 0.6589 0.5] Start depleting wellness
  (bind _returnvalue (`KismetSystemLibrary.K2_SetTimerDelegate` (delegate `depleteWellness`) 1.0 true))
  (set `self.wellnessDepletionTimer` _returnvalue))

(event `stopWellnessDepletion`
  ;[1 0.3388 0.6589 0.5] Stop depleting wellness
  (`KismetSystemLibrary.K2_ClearAndInvalidateTimerHandle` (`self.wellnessDepletionTimer`)))

(event `self.ReceiveBeginPlay`
  ;[1 0.3388 0.6589 0.5] Depletion Event Binding
  (bind _returnvalue (`GameplayStatics.GetActorOfClass` "/Game/FirstPerson/Blueprints/BP_FirstPersonCharacter.BP_FirstPersonCharacter_C"))
  (add `/Game/FirstPerson/Blueprints/BP_FirstPersonCharacter.onStartHealthDepletion` _returnvalue (delegate `handleWellnessDepletion`))
  (add `/Game/FirstPerson/Blueprints/BP_FirstPersonCharacter.onStopHealthDepletion` _returnvalue (delegate `handleDepletionStop`))
  ;[1 0.3388 0.6589 0.5] Bind Update Depletion Rate (Difficulty) and Update wellness' for days
  (bind _returnvalue_2 (`GameplayStatics.GetActorOfClass` "/Game/BP_Bed.BP_Bed_C"))
  (bind _bed (message `/Game/DarcyBlueprints/BPI_UpdateDay.getBed` _returnvalue_2))
  (add `/Game/BP_Bed.onPlayerSleep` _bed (delegate `updateDepletionRate`))
  (bind _returnvalue_3 (`GameplayStatics.GetActorOfClass` "/Game/BP_Bed.BP_Bed_C"))
  (bind _day (message `/Game/DarcyBlueprints/BPI_UpdateDay.updateDay` _returnvalue_3))
  (switch `int` _day
    (:`Default`
      (set `self.maxWellness` 100.0)
      (set `self.minWellness` 0.0))
    (:`1`
      (set `self.maxWellness` 50.0)
      (set `self.minWellness` 1.0 :!label _label))
    (:`2`
      (set `self.maxWellness` 75.0)
      (goto _label))))

(event `updateDepletionRate`
  ;[1 0.3388 0.6589 0.5] Bind Update Depletion Rate (Difficulty) and Update wellness' for days
  (bind _day (message `/Game/DarcyBlueprints/BPI_UpdateDay.updateDay` (stale `self.ReceiveBeginPlay` _bed)))
  (`self.resetWellness`)
  (switch `int` _day
    (:`Default`
      (set `self.depletionRate` 1.0))
    (:`5`
      (set `self.depletionRate` 2.0))
    (:`6`
      (set `self.depletionRate` 3.0))))

(event `depleteWellness`
  ;[1 0.3388 0.6589 0.5] Deplete wellness logic
  (if (`self.ActorHasTag` "Main")
    (if (`self.dead`)
      _
      (elif (not (`self.playerFire`))
        (set `self.wellness` (`KismetMathLibrary.FClamp` (- (`self.wellness`) (`self.depletionRate`)) 0.0 100.0))
        (if (== (`self.wellness`) 0.0)
          (bind _returnvalue (`GameplayStatics.GetActorOfClass` "/Game/FirstPerson/Blueprints/BP_FirstPersonCharacter.BP_FirstPersonCharacter_C"))
          (`/Game/FirstPerson/Blueprints/BP_FirstPersonCharacter.OnDead` _returnvalue)
          (set `self.dead` true)
          (else
            (`self.updateThreshold`)))))))

(event `resetWellness`
  ;[1 0.3388 0.6589 0.5] On New Day, Reset Wellness
  (if (`self.ActorHasTag` "Main")
    (set `self.wellness` 100.0)))

(event `updateThreshold`
  ;[1 0.3388 0.6589 0.5] Updates current threshold
  (for (_array_element _array_index) (`self.wellnessThresholds`)
    (set `self.lowerThreshold` _array_element)
    (bind _result (`/Engine/EditorBlueprintResources/StandardMacros.IncrementFloat` _array_element)
      (:`  `
        (set `self.upperThreshold` _result)
        (if (and (>= (`self.wellness`) (`self.lowerThreshold`)) (< (`self.wellness`) (`self.upperThreshold`)))
          (set `self.currentThreshold` _array_index)
          (`self.updateMesh`)
          (break))))))

(event `updateMesh`
  ;[1 0.3388 0.6589 0.5] Updates Meshes depending on wellness
  (switch `int` (`self.currentThreshold`)
    (:`0`
      (set `self.currentMesh` (`self.smallMesh`)))
    (:`1`
      (set `self.currentMesh` (`self.mediumMesh`)))
    (:`2`
      (set `self.currentMesh` (`self.largeMesh`))))
  (`StaticMeshComponent.SetStaticMesh` (`self.factorMesh`) (`self.currentMesh`)))

(fn `getBed`
  (returns (bed :type "/Game/BP_Bed Object Reference"))
  (return null))

(fn `updateDay`
  (returns (day :type Integer))
  (return 0))

(fn `UserConstructionScript`
  (bind _factorinfo (`self.factorInfo`))
  (bind _factormesh (`self.factorMesh`))
  ;[1 0.3388 0.6589 0.5] Setting Blueprint to have assigned Tool Data Asset values
  (set `self.largeMesh` (`/Game/DarcyBlueprints/DataAssets/BP_FactorDABase.LargeMesh` _factorinfo))
  (set `self.smallMesh` (`/Game/DarcyBlueprints/DataAssets/BP_FactorDABase.SmallMesh` _factorinfo))
  (set `self.mediumMesh` (`/Game/DarcyBlueprints/DataAssets/BP_FactorDABase.MediumMesh` _factorinfo))
  (set `self.factor` (`/Game/DarcyBlueprints/DataAssets/BP_FactorDABase.Factor` _factorinfo))
  (if (`self.ActorHasTag` "Tutorial")
    (set `self.wellness` 1.0)
    (`StaticMeshComponent.SetStaticMesh` _factormesh (`self.smallMesh`))
    (else
      (set `self.wellness` 1.0)
      (`StaticMeshComponent.SetStaticMesh` _factormesh (`self.largeMesh`)))))