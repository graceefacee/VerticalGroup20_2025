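; BP_ToolBase is a base tool Blueprint that changes the wellness of hit actors according to their Factor.
; Its construction script copies name, description, factors, effects and mesh from a ToolInfo data asset.
; ApplyEffect passes PosEffect to ModifyWellness on PosFactor matches; NegFactor matches log NegEffect but pass zero.
; GetTool returns ToolInfo, while GetFactor returns a fixed enum value.
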(event `/Game/DarcyBlueprints/BPI_HitEffect.applyEffect`
  (params (hitActors :type "Array of /Game/DarcyBlueprints/Factors/BP_FactorBase Object Reference (by ref)"))
  (bind _poseffect (`self.posEffect`))
  ;[1 0.3388 0.6589 0.5] Gets Hit Actors, for each, it checks if it is effected (Positively or Negatively) then sends the appropriate effects value to the factor
  (for _array_element hitActors
    (bind _factor (`/Game/DarcyBlueprints/Factors/BP_FactorBase.factor` _array_element))
    (if (`|EnumEquality` (`self.posFactor`) _factor)
      (`/Game/DarcyBlueprints/BPI_UpdateFactor.modifyWellness` _array_element _poseffect)
      (`KismetSystemLibrary.LogString` (`KismetStringLibrary.Conv_DoubleToString` _poseffect))
      (elif (`|EnumEquality` _factor (`self.negFactor`))
        (`/Game/DarcyBlueprints/BPI_UpdateFactor.modifyWellness` _array_element 0.0)
        (`KismetSystemLibrary.LogString` (`KismetStringLibrary.Conv_DoubleToString` (`self.negEffect`)))))))

(fn `getFactor`
  (returns (Factor :type "/Game/DarcyBlueprints/Factors/E_EnvFactorTypes Enum"))
  (return "NewEnumerator0"))

(fn `getTool`
  (returns (toolInfo :type "/Game/DarcyBlueprints/DataAssets/BP_ToolDABase Object Reference"))
  (return (`self.toolInfo`)))

(fn `UserConstructionScript`
  (locals (NewLocalVar :type "StaticMeshComponent Object Reference"))
  (bind _toolinfo (`self.toolInfo`))
  ;[1 0.3388 0.6589 0.5] Setting Blueprint to have assigned Tool Data Asset values
  (set `self.name` (`/Game/DarcyBlueprints/DataAssets/BP_ToolDABase.Name` _toolinfo))
  (set `self.description` (`/Game/DarcyBlueprints/DataAssets/BP_ToolDABase.Description` _toolinfo))
  (set `self.posFactor` (`/Game/DarcyBlueprints/DataAssets/BP_ToolDABase.PosFactor` _toolinfo))
  (set `self.negFactor` (`/Game/DarcyBlueprints/DataAssets/BP_ToolDABase.NegFactor` _toolinfo))
  (set `self.posEffect` (`/Game/DarcyBlueprints/DataAssets/BP_ToolDABase.PosEffect` _toolinfo))
  (set `self.negEffect` (`/Game/DarcyBlueprints/DataAssets/BP_ToolDABase.NegEffect` _toolinfo))
  (`StaticMeshComponent.SetStaticMesh` (`self.toolMesh`) (`/Game/DarcyBlueprints/DataAssets/BP_ToolDABase.Mesh` _toolinfo)))