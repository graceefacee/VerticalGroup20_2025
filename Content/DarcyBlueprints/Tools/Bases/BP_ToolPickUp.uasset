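; BP_ToolPickUp is a tool pickup actor that shows the tool's name when the player gets near it.
; The ToolInfo struct supplies the mesh set in the construction script and the name sent to the WBP_PickUp widget.
; Sphere overlap with BP_FirstPersonCharacter shows the prompt, and any end overlap hides it.
; GetTool exposes ToolInfo, while UpdateDay is a stub returning zero; the pickup action itself is not handled here.
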(event `self.Sphere.OnComponentBeginOverlap`
  (params (OverlappedComponent :type "PrimitiveComponent Object Reference") (OtherActor :type "Actor Object Reference") (OtherComp :type "PrimitiveComponent Object Reference") (OtherBodyIndex :type Integer) (bFromSweep :type Boolean) (SweepResult :type "HitResult Structure (by ref)"))
  ;[1 0.3388 0.6589 0.5] When approaching tool, pick up text appears
  (if (== (`GameplayStatics.GetObjectClass` OtherActor) "/Game/FirstPerson/Blueprints/BP_FirstPersonCharacter.BP_FirstPersonCharacter_C")
    (`self.getTool`)
    (bind _aswbp_pick_up (cast `/Game/DarcyBlueprints/UI/WBP_PickUp` (`WidgetComponent.GetWidget` (`self.PickUpText`))))
    (`/Game/DarcyBlueprints/UI/WBP_PickUp.updateName` _aswbp_pick_up (`/Game/DarcyBlueprints/DataAssets/BP_ToolDABase.Name` (`self.toolInfo`)))
    (`SceneComponent.SetVisibility` (`self.PickUpText`) true false)))

(event `self.Sphere.OnComponentEndOverlap`
  (params (OverlappedComponent :type "PrimitiveComponent Object Reference") (OtherActor :type "Actor Object Reference") (OtherComp :type "PrimitiveComponent Object Reference") (OtherBodyIndex :type Integer))
  ;[1 0.3388 0.6589 0.5] When approaching tool, pick up text appears
  (`SceneComponent.SetVisibility` (`self.PickUpText`) false false))

(fn `getTool`
  (returns (toolInfo :type "/Game/DarcyBlueprints/DataAssets/BP_ToolDABase Object Reference"))
  (return (`self.toolInfo`)))

(fn `updateDay`
  (returns (day :type Integer))
  (return 0))

(fn `UserConstructionScript`
  (`StaticMeshComponent.SetStaticMesh` (`self.toolMesh`) (`/Game/DarcyBlueprints/DataAssets/BP_ToolDABase.Mesh` (`self.toolInfo`))))