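; BP_ToolSpawner places tools in the level on the day they unlock, moving existing actors rather than spawning new ones.
; On BeginPlay it finds BP_Bed, binds to its player-sleep event and runs an initial placement pass.
; Each pass gets the day from the bed and teleports tools with a matching UnlockDay to spawn points tagged with that tool's first tag.
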(event `self.ReceiveBeginPlay`
  (bind _returnvalue (`GameplayStatics.GetActorOfClass` "/Game/BP_Bed.BP_Bed_C"))
  (bind _bed (message `/Game/DarcyBlueprints/BPI_UpdateDay.getBed` _returnvalue))
  (add `/Game/BP_Bed.onPlayerSleep` _bed (delegate `spawnTool`))
  (`self.spawnTool`))

(event `spawnTool`
  (bind _day (message `/Game/DarcyBlueprints/BPI_UpdateDay.updateDay` (stale `self.ReceiveBeginPlay` _returnvalue)))
  (for _array_element (`self.tools`)
    (if (== _day (`/Game/DarcyBlueprints/DataAssets/BP_ToolDABase.unlockDay` (`/Game/DarcyBlueprints/Tools/Bases/BP_ToolPickUp.toolInfo` _array_element)))
      (for _array_element_2 (`self.spawnPoints`)
        (if (`self.ActorHasTag` _array_element_2 (`|GetArrayItem` (`Actor.Tags` _array_element)))
          (`self.K2_SetActorTransform` _array_element (`self.GetTransform` _array_element_2) false true))))))

(fn `getBed`
  (returns (bed :type "/Game/BP_Bed Object Reference"))
  (return null))

(fn `updateDay`
  (returns (day :type Integer))
  (return 0))

(fn `UserConstructionScript`)