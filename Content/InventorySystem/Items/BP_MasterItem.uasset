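; BP_MasterItem is an inventory item actor that the first-person character picks up with the E key.
; Overlapping its collision component caches the BP_FirstPersonCharacter and enables input on the item for player controller 0, and ending any overlap disables it.
; Pressing E passes ItemInfo to the character's PickItem and destroys the actor, without checking whether the pickup succeeded.
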(event `Key|E`
  (params (Key :type "Key Structure"))
  (:`Pressed`
    (`/Game/FirstPerson/Blueprints/BP_FirstPersonCharacter.PickItem` (`self.CharacterCast`) (`self.ItemInfo`))
    (`self.K2_DestroyActor`)))

(event `self.Collision.OnComponentBeginOverlap`
  (params (OverlappedComponent :type "PrimitiveComponent Object Reference") (OtherActor :type "Actor Object Reference") (OtherComp :type "PrimitiveComponent Object Reference") (OtherBodyIndex :type Integer) (bFromSweep :type Boolean) (SweepResult :type "HitResult Structure (by ref)"))
  ;[0.04667 0.15 0.0382 0.502] Collision Input
  (bind _asbp_first_person_character (cast `/Game/FirstPerson/Blueprints/BP_FirstPersonCharacter` OtherActor))
  (set `self.CharacterCast` _asbp_first_person_character)
  (`self.EnableInput` (`GameplayStatics.GetPlayerController` 0)))

(event `self.Collision.OnComponentEndOverlap`
  (params (OverlappedComponent :type "PrimitiveComponent Object Reference") (OtherActor :type "Actor Object Reference") (OtherComp :type "PrimitiveComponent Object Reference") (OtherBodyIndex :type Integer))
  ;[0.04667 0.15 0.0382 0.502] Collision Input
  (`self.DisableInput` (`GameplayStatics.GetPlayerController` 0)))

(fn `UserConstructionScript`)